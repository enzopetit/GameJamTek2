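; BP_FlammeReceiver is an interactable receiver that takes the flame the player carries and lights itself.
; A sphere overlap shows or hides a widget while something is in range.
; Interact reveals the cone meshes and Niagara flame, plays a fire sound, hides the third-person character's flames and disables the sphere's collision.
; It then calls EndLocation on GrandePorte, apparently a large door.
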(event `self.Sphere.OnComponentBeginOverlap`
  (params (OverlappedComponent :type "PrimitiveComponent Object Reference") (OtherActor :type "Actor Object Reference") (OtherComp :type "PrimitiveComponent Object Reference") (OtherBodyIndex :type Integer) (bFromSweep :type Boolean) (SweepResult :type "HitResult Structure (by ref)"))
  (`SceneComponent.SetVisibility` (`self.Widget`) true false))

(event `self.Sphere.OnComponentEndOverlap`
  (params (OverlappedComponent :type "PrimitiveComponent Object Reference") (OtherActor :type "Actor Object Reference") (OtherComp :type "PrimitiveComponent Object Reference") (OtherBodyIndex :type Integer))
  (`SceneComponent.SetVisibility` (`self.Widget`) false false))

(event `/Game/Blueprints/Interfaces/BPI_Interact.Interact`
  (`SceneComponent.SetVisibility` (`self.Cone`) true false)
  (`SceneComponent.SetVisibility` (`self.Cone1`) true false)
  (`SceneComponent.SetVisibility` (`self.NS_Flamme`) true false)
  (`GameplayStatics.PlaySoundAtLocation` "/Game/Sons/FIREBurn_Grand_feu_de_branches_1__ID_0987__LS.FIREBurn_Grand_feu_de_branches_1__ID_0987__LS" (`self.K2_GetActorLocation`) (struct) 1.0 1.0 0.0 "/Game/Sons/SA_Fire.SA_Fire" null null null)
  (bind _asbp_third_person_character (cast `/Game/ThirdPerson/Blueprints/BP_ThirdPersonCharacter` (`GameplayStatics.GetPlayerCharacter` 0)))
  (`SceneComponent.SetVisibility` (`/Game/ThirdPerson/Blueprints/BP_ThirdPersonCharacter.Flamme1` _asbp_third_person_character) false false)
  (`SceneComponent.SetVisibility` (`/Game/ThirdPerson/Blueprints/BP_ThirdPersonCharacter.Flamme` _asbp_third_person_character) false false)
  (`PrimitiveComponent.SetCollisionEnabled` (`self.Sphere`) "NoCollision")
  (`/Game/Blueprints/Actors/BP_GrandePorte.EndLocation` (`self.GrandePorte`)))

(fn `UserConstructionScript`)