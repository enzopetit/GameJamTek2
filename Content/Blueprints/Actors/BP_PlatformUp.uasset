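; BP_PlatformUp is a platform actor that shuttles endlessly between its placed location and an offset, starting on BeginPlay.
; It stores its starting location, then each Timeline_0 update adds the track value to it and sets the actor's location without sweep.
; When the timeline finishes, its direction selects StartLocation to reverse from the end or EndLocation to play from the start, forming a ping-pong loop.
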(event `self.ReceiveBeginPlay`
  (set `self.StarLocation` (`self.K2_GetActorLocation`))
  (`self.EndLocation`))

(event `StartLocation`
  (bind (_direction _newtrack_0) (`Timeline|Timeline_0` :!via `ReverseFromEnd` :!label _label)
    (:`Update`
      (`self.K2_SetActorLocation` (+ (`self.StarLocation`) _newtrack_0)))
    (:`Finished`
      (switch `ETimelineDirection` _direction
        (:`Forward`
          (`self.StartLocation`))
        (:`Backward`
          (`self.EndLocation`))))))

(event `EndLocation`
  (goto _label :!via `PlayFromStart`))

(fn `UserConstructionScript`)